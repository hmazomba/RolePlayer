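; Enemy character Blueprint that drives combat AI against a locked target.
; ToggleAttackMode loops a FlipFlop between timed attack phases and shorter strafe phases with random blocking and strafe direction.
; ToggleAttacking repeats AIAttack at random intervals, first sending the AI controller toward the target when out of hit range.
; While not attacking, Tick-driven CombatStrafing moves sideways and forward or back around a distance threshold, using control yaw only.
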(event `self.ReceiveTick`
  (params (DeltaSeconds :type "Float (single-precision)"))
  (bind _returnvalue (`KismetMathLibrary.MakeRotator` 0.0 0.0 (.yaw (`self.GetControlRotation`))))
  (`parent.ReceiveTick` DeltaSeconds)
  (`/Engine/EditorBlueprintResources/StandardMacros.IsValid` (`self.LockedEnemy`)
    (:`Is Valid`
      (if (not (`self.IsAttacking`))
        (`self.AddMovementInput` (`KismetMathLibrary.GetRightVector` _returnvalue) (`self.CombatStrafe`))
        (`self.AddMovementInput` (`KismetMathLibrary.GetForwardVector` _returnvalue) (select `bool` (> (`self.GetDistanceTo` (`self.LockedEnemy`) self) 500.0) :`false` -1.0 :`true` 1.0 :!type "Float (single-precision)"))))))

(event `self.ToggleAttacking`
  (params (Enable :type Boolean) (Enemy :type "Actor Object Reference"))
  (bind _returnvalue (`self.K2_GetActorLocation` Enemy))
  ;[0.9922 0 1] NPC Attack loop
  (bind _output_get (set `self.IsAttacking` Enable))
  (if _output_get
    (`/Engine/EditorBlueprintResources/StandardMacros.DoOnce` false :!label _label
      (:`Completed`
        (`/Engine/EditorBlueprintResources/StandardMacros.IsValid` Enemy :!label _label_2
          (:`Is Valid`
            (if (not (< (`self.GetDistanceTo` Enemy self) (`self.HitRange`)))
              (`AIController.MoveToLocation` (`AIBlueprintHelperLibrary.GetAIController` self) (+ (* (`KismetMathLibrary.Normal` (- (`self.K2_GetActorLocation`) _returnvalue)) (* (`self.HitRange`) 0.6)) _returnvalue) 10.0 true true true true null true)
              (`KismetSystemLibrary.Delay` 2.5))
            (`self.AIAttack`)
            (`KismetSystemLibrary.Delay` (`KismetMathLibrary.RandomFloatInRange` 1.5 3.5))
            (if (`self.IsAttacking`)
              (goto _label_2)
              (else
                (goto _label :!via `Reset`)))))))))

(event `self.ToggleAttackMode`
  (params (Enable :type Boolean) (Enemy :type "Actor Object Reference"))
  (set `self.LockedEnemy` Enemy)
  (bind _output_get (set `self.InAttackMode?` Enable))
  (if _output_get
    (`/Engine/EditorBlueprintResources/StandardMacros.DoOnce` false
      (:`Completed`
        (`/Engine/EditorBlueprintResources/StandardMacros.FlipFlop` :!label _label_3
          (:`A`
            ;[0 1 0.3906] AI Attack
            (set `self.CombatStrafe` 0.0)
            (`self.ToggleAttacking` true (`self.LockedEnemy`))
            (`KismetSystemLibrary.Delay` (`KismetMathLibrary.RandomFloatInRange` 6.0 12.0)))
          (:`B`
            (`self.ToggleBlock` (`KismetMathLibrary.RandomBool`))
            ;[0 1 0.3672] Strafe
            (set `self.CombatStrafe` (`KismetMathLibrary.RandomFloatInRange` -0.5 0.5))
            (`self.ToggleAttacking` false)
            (`KismetSystemLibrary.Delay` (`KismetMathLibrary.RandomFloatInRange` 2.0 3.0))))
        (if (`self.InAttackMode?`)
          (goto _label_3))))
    (else
      (`self.ToggleAttacking` false))))

(fn `UserConstructionScript`
  (`parent.UserConstructionScript`))